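; BP_AITankPawn is an AI tank pawn Blueprint that displays its health in an attached widget.
; On BeginPlay it casts the WidgetHP user widget to WBP_AI_HP and sets the AIHealthPoint bar to HealthComponent's current-to-max health ratio.
; MyBPEvent repeats the same update to refresh the bar, with no caller shown in this Blueprint.
; The construction script only calls its parent.
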(event `self.ReceiveBeginPlay`
  (bind _healthcomponent (`self.HealthComponent`))
  ;[1 1 1] Установка ХП при старте игры
  (bind _aswbp_ai_hp (cast `/Game/UI/Widgets/WBP_AI_HP` (`WidgetComponent.GetUserWidgetObject` (`self.Widget_HP`))))
  (`ProgressBar.SetPercent` (`/Game/UI/Widgets/WBP_AI_HP.AI_HealthPoint` _aswbp_ai_hp) (/ (`HealthComponent.CurrentHealth` _healthcomponent) (`HealthComponent.MaxHealth` _healthcomponent))))

(event `self.MyBPEvent`
  (bind _healthcomponent (`self.HealthComponent`))
  ;[1 1 1] Обновление ХП.
  (bind _aswbp_ai_hp (cast `/Game/UI/Widgets/WBP_AI_HP` (`WidgetComponent.GetUserWidgetObject` (`self.Widget_HP`))))
  (`ProgressBar.SetPercent` (`/Game/UI/Widgets/WBP_AI_HP.AI_HealthPoint` _aswbp_ai_hp) (/ (`HealthComponent.CurrentHealth` _healthcomponent) (`HealthComponent.MaxHealth` _healthcomponent))))

(fn `UserConstructionScript`
  (`parent.UserConstructionScript`))